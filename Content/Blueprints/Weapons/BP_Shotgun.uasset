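; BP_Shotgun is a weapon Blueprint whose Shoot function fires a spread of pellet projectiles.
; It loops on a pellet count, spawning double-scale BP_Bullet actors at the Scene component, each with random roll, pitch and yaw offsets within Spread.
; Each bullet receives the weapon's speed and damage, then one fire sound plays at the actor's location.
; The event graph and construction script contain no logic.
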(event `self.ReceiveBeginPlay`)

(event `self.ReceiveTick`
  (params (DeltaSeconds :type "Float (single-precision)")))

(fn `Shoot`
  (bind _spread (`self.Spread`))
  (bind (_returnvalue_location _returnvalue_rotation) (`KismetMathLibrary.BreakTransform` (`SceneComponent.K2_GetComponentToWorld` (`self.Scene`))))
  (bind _returnvalue (- 0.0 _spread))
  (for _ (range (+ (`self.iPellets`) 1))
    (bind _returnvalue_2 (`|SpawnActorFromClass` "/Game/Blueprints/Weapons/Bullets/BP_Bullet.BP_Bullet_C" (`KismetMathLibrary.MakeTransform` _returnvalue_location (`KismetMathLibrary.MakeRotator` (+ (.roll _returnvalue_rotation) (`KismetMathLibrary.RandomFloatInRange` _returnvalue _spread)) (+ (.pitch _returnvalue_rotation) (`KismetMathLibrary.RandomFloatInRange` _returnvalue _spread)) (+ (.yaw _returnvalue_rotation) (`KismetMathLibrary.RandomFloatInRange` _returnvalue _spread))) (2.0 2.0 2.0)) "Undefined" "OverrideRootScale" null null))
    (set `/Game/Blueprints/Weapons/Bullets/BP_Bullet.Speed` (`self.BulletSpeed`) _returnvalue_2)
    (set `/Game/Blueprints/Weapons/Bullets/BP_Bullet.Damage` (`self.Damage`) _returnvalue_2))
  (`GameplayStatics.PlaySoundAtLocation` "/Game/Assets/Audio/Audio/SoundEffects/Weapons/FirstPersonTemplateWeaponFire02.FirstPersonTemplateWeaponFire02" (`self.K2_GetActorLocation`) (struct) 1.0 1.0 0.0 null null null))

(fn `UserConstructionScript`)