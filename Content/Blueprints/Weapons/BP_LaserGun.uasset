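; Laser gun weapon Blueprint that fires a continuous beam, tracing and applying damage every Tick while Shooting is true.
; Shoot line-traces on Visibility from the Scene component along its forward vector for LaserLength, with debug drawing.
; The Laser beam runs from Scene to the hit point or trace end, and hit actors receive damage.
; LaserOff hides the beam; Shoot's visibility check also sets it hidden, so neither shows it.
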(event `self.ReceiveBeginPlay`)

(event `self.ReceiveTick`
  (params (DeltaSeconds :type "Float (single-precision)"))
  (if (`self.Shooting`)
    (`self.Shoot`)))

(fn `LaserOff`
  (`SceneComponent.SetVisibility` (`self.Laser`) false false))

(fn `Shoot`
  (bind _laser (`self.Laser`))
  (bind _scene (`self.Scene`))
  (bind _laser_2 (`self.Laser`))
  (bind _returnvalue (`SceneComponent.K2_GetComponentLocation` _scene))
  ;[1 1 1] Set Visible
  (if (not (== (`SceneComponent.IsVisible` _laser_2) true))
    (`SceneComponent.SetVisibility` _laser_2 false false))
  ;[1 1 1] Raycast
  (`ParticleSystemComponent.SetBeamSourcePoint` _laser 0 _returnvalue 0)
  (bind (_outhit _returnvalue_2) (`KismetSystemLibrary.LineTraceSingle` :`Start` _returnvalue :`End` (+ _returnvalue (* (`SceneComponent.GetForwardVector` _scene) (`self.LaserLength`))) :`TraceChannel` "TraceTypeQuery1" :`DrawDebugType` "ForOneFrame"))
  (if _returnvalue_2
    (bind (_bblockinghit _binitialoverlap _time _distance _location _impactpoint _normal _impactnormal _physmat _hitactor _hitcomponent _hitbonename _hititem _faceindex _tracestart _traceend) (`GameplayStatics.BreakHitResult` _outhit))
    ;[1 1 1] Set Beem Target
    (`ParticleSystemComponent.SetBeamTargetPoint` _laser 0 _location 0)
    ;[1 1 1] Damage Target
    (`GameplayStatics.ApplyDamage` _hitactor)
    (else
      (`ParticleSystemComponent.SetBeamTargetPoint` _laser 0 _traceend 0))))

(fn `UserConstructionScript`)