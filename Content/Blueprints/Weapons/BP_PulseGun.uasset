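; BP_PulseGun is a charge-up weapon that fires a BP_Bullet scaled by the stored charge.
; IsShooting sets the firing state and starts or stops a looping charge sound.
; While firing, Tick builds clamped charge through a short Delay and blends two point lights from red to green.
; Once released with at least minimum charge, Tick calls Shoot, which spawns the bullet, plays a fire sound and resets charge and lights.
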(event `self.ReceiveBeginPlay`)

(event `self.ReceiveTick`
  (params (DeltaSeconds :type "Float (single-precision)"))
  (bind _returnvalue (/ (`self.CurrentChargeAmount`) (`self.FullChrage`)))
  (if (`self.Shooting`)
    (`KismetSystemLibrary.Delay` 0.05)
    (set `self.CurrentChargeAmount` (`KismetMathLibrary.FClamp` (+ (`self.CurrentChargeAmount`) 0.05) 0.0 (`self.FullChrage`)))
    (`LightComponent.SetLightColor` (`self.PointLight`) (make `LinearColor` (- 1.0 _returnvalue) _returnvalue) true)
    (`LightComponent.SetLightColor` (`self.PointLight1`) (make `LinearColor` (- 1.0 _returnvalue) _returnvalue) true)
    (elif (>= (`self.CurrentChargeAmount`) (`self.MinCharge`))
      (`self.Shoot`))))

(fn `ChrageUp`)

(fn `IsShooting`
  (params (bShooting :type Boolean))
  (bind _chrageupsound (`self.ChrageUpSound`))
  (bind _output_get (set `self.Shooting` bShooting))
  (if _output_get
    (bind _returnvalue (`GameplayStatics.SpawnSoundAttached` "/Game/Assets/Audio/Audio/Loops/Endless_Rising_-_Loop.Endless_Rising_-_Loop" (`self.StaticMesh`) "None" (0.0 0.0 0.0) (struct) "KeepRelativeOffset" false 1.0 1.0 0.0 null null))
    (set `self.ChrageUpSound` _returnvalue)
    (else
      (`/Engine/EditorBlueprintResources/StandardMacros.IsValid` _chrageupsound
        (:`Is Valid`
          (`AudioComponent.Stop` _chrageupsound)
          (`ActorComponent.K2_DestroyComponent` _chrageupsound))))))

(fn `Shoot`
  (bind (_returnvalue_location _returnvalue_rotation) (`KismetMathLibrary.BreakTransform` (`SceneComponent.K2_GetComponentToWorld` (`self.Scene`))))
  (bind _returnvalue (* (/ (`self.CurrentChargeAmount`) (`self.FullChrage`)) 10.0))
  (bind _returnvalue_2 (`|SpawnActorFromClass` "/Game/Blueprints/Weapons/BP_Bullet.BP_Bullet_C" (`KismetMathLibrary.MakeTransform` _returnvalue_location _returnvalue_rotation (`KismetMathLibrary.MakeVector` _returnvalue _returnvalue _returnvalue)) "Undefined" "OverrideRootScale" null null))
  (set `/Game/Blueprints/Weapons/BP_Bullet.Speed` 10.0 _returnvalue_2)
  (`GameplayStatics.PlaySoundAtLocation` "/Game/Assets/Audio/Audio/SoundEffects/Weapons/FirstPersonTemplateWeaponFire02.FirstPersonTemplateWeaponFire02" (`self.K2_GetActorLocation`) (struct) 1.0 1.0 0.0 null null null)
  (set `self.CurrentChargeAmount` 0.0)
  (`LightComponent.SetLightColor` (`self.PointLight`) (make `LinearColor` 1.0) true)
  (`LightComponent.SetLightColor` (`self.PointLight1`) (make `LinearColor` 1.0) true))

(fn `UserConstructionScript`)