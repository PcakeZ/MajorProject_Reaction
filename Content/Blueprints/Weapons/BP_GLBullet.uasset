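; BP_GLBullet is an explosive projectile, apparently a grenade launcher round, that deals radial damage when it detonates.
; BeginPlay starts an auto-detonate delay, and the ExplodeGrenade event jumps into the same detonation chain to skip the wait.
; Detonation spawns an explosion emitter and sound at the Sphere component, applies radial damage with itself as causer, then destroys the actor.
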(event `self.ReceiveBeginPlay`
  (bind (_returnvalue_location _returnvalue_rotation) (`KismetMathLibrary.BreakTransform` (`SceneComponent.K2_GetComponentToWorld` (`self.Sphere`))))
  (`KismetSystemLibrary.Delay` (`self.AutoDetonateTimer`))
  (`GameplayStatics.SpawnEmitterAtLocation` "/Game/StarterContent/Particles/P_Explosion.P_Explosion" _returnvalue_location _returnvalue_rotation :!label _label)
  (`GameplayStatics.PlaySoundAtLocation` "/Game/Assets/Audio/Audio/SoundEffects/Weapons/FirstPersonTemplateWeaponFire02.FirstPersonTemplateWeaponFire02" _returnvalue_location (struct) 1.0 1.0 0.0 null null null)
  ;[1 1 1] Damage Enemies
  (`GameplayStatics.ApplyRadialDamage` :`BaseDamage` (`self.BaseDamage`) :`Origin` (`SceneComponent.K2_GetComponentLocation` (`self.Sphere`)) :`DamageRadius` (`self.DamageRadius`) :`DamageTypeClass` "/Script/Engine.DamageType" :`DamageCauser` self :`InstigatedByController` null)
  (`self.K2_DestroyActor`))

(event `/Game/Blueprints/Interface/I_GrenadeLauncher.ExplodeGrenade`
  (goto _label))

(fn `UserConstructionScript`)