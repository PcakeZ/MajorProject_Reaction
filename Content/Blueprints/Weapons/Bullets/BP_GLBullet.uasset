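; BP_GLBullet is a grenade launcher projectile that explodes and deals radial damage.
; It detonates after an auto-detonate timer, when the ExplodeGrenade event is called, or when its Sphere1 trigger overlaps an actor implementing I_Enemy.
; Explode spawns an explosion emitter and sound at the Sphere's location, applies radial damage from there, then destroys the actor.
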(event `self.ReceiveBeginPlay`
  (`KismetSystemLibrary.Delay` (`self.AutoDetonateTimer`))
  (`self.Explode` :!label _label))

(event `/Game/Blueprints/Interface/I_GrenadeLauncher.ExplodeGrenade`
  (goto _label))

(event `self.Sphere1.OnComponentBeginOverlap`
  (params (OverlappedComponent :type "PrimitiveComponent Object Reference") (OtherActor :type "Actor Object Reference") (OtherComp :type "PrimitiveComponent Object Reference") (OtherBodyIndex :type Integer) (bFromSweep :type Boolean) (SweepResult :type "HitResult Structure (by ref)"))
  (if (`KismetSystemLibrary.DoesImplementInterface` OtherActor "/Game/Blueprints/Interface/I_Enemy.I_Enemy_C")
    (`self.Explode`)))

(fn `Explode`
  (bind (_returnvalue_location _returnvalue_rotation) (`KismetMathLibrary.BreakTransform` (`SceneComponent.K2_GetComponentToWorld` (`self.Sphere`))))
  (`GameplayStatics.SpawnEmitterAtLocation` "/Game/StarterContent/Particles/P_Explosion.P_Explosion" _returnvalue_location _returnvalue_rotation)
  (`GameplayStatics.PlaySoundAtLocation` "/Game/Assets/Audio/Audio/SoundEffects/Weapons/FirstPersonTemplateWeaponFire02.FirstPersonTemplateWeaponFire02" _returnvalue_location (struct) 1.0 1.0 0.0 null null null)
  ;[1 1 1] Damage Enemies
  (`GameplayStatics.ApplyRadialDamage` :`BaseDamage` (`self.BaseDamage`) :`Origin` (`SceneComponent.K2_GetComponentLocation` (`self.Sphere`)) :`DamageRadius` (`self.DamageRadius`) :`DamageTypeClass` "/Script/Engine.DamageType" :`DamageCauser` self :`InstigatedByController` null)
  (`self.K2_DestroyActor`))

(fn `UserConstructionScript`)