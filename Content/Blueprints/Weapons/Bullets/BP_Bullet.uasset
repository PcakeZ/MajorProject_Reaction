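; BP_Bullet is a projectile that damages melee and crawler AI enemies.
; Tick teleports it along its forward vector by Speed each frame, without sweeping or delta-time scaling, so its speed depends on frame rate.
; A capsule overlap with BP_MeleeAI or BP_CrawlAI applies damage and destroys the bullet, while other actors are ignored.
; BeginPlay destroys it after a fixed lifetime if it hits neither.
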(event `self.ReceiveBeginPlay`
  (`KismetSystemLibrary.Delay` 8.0)
  (`self.K2_DestroyActor`))

(event `self.ReceiveTick`
  (params (DeltaSeconds :type "Float (single-precision)"))
  (`self.K2_SetActorLocation` (+ (`self.K2_GetActorLocation`) (* (`KismetMathLibrary.GetForwardVector` (`self.K2_GetActorRotation`)) (`self.Speed`)))))

(event `self.Capsule.OnComponentBeginOverlap`
  (params (OverlappedComponent :type "PrimitiveComponent Object Reference") (OtherActor :type "Actor Object Reference") (OtherComp :type "PrimitiveComponent Object Reference") (OtherBodyIndex :type Integer) (bFromSweep :type Boolean) (SweepResult :type "HitResult Structure (by ref)"))
  (bind _asbp_melee_ai (cast `/Game/Blueprints/Enemies/Melee/BP_MeleeAI` OtherActor)
    (:`then`
      (`GameplayStatics.ApplyDamage` _asbp_melee_ai 1.0 null null "/Script/Engine.DamageType"))
    (:`CastFailed`
      (bind _asbp_crawl_ai (cast `/Game/Blueprints/Enemies/Melee/BP_CrawlAI` OtherActor))
      (`GameplayStatics.ApplyDamage` _asbp_crawl_ai 1.0 null null "/Script/Engine.DamageType")))
  (`self.K2_DestroyActor`))

(fn `UserConstructionScript`)