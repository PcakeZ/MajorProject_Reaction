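; BP_SMG is an automatic submachine gun that fires bullets repeatedly while its Shooting flag is set.
; IsShooting sets that flag, and Tick uses a Delay of FireRate to pace each call to Shoot, so the first shot also waits.
; Shoot spawns an enlarged BP_Bullet at the Scene component, passes it BulletSpeed and Damage, and plays the SMG sound at the weapon's location.
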(event `self.ReceiveBeginPlay`)

(event `self.ReceiveTick`
  (params (DeltaSeconds :type "Float (single-precision)"))
  (if (`self.Shooting`)
    (`KismetSystemLibrary.Delay` (`self.FireRate`))
    (`self.Shoot`)))

(fn `IsShooting`
  (params (bShooting :type Boolean))
  (set `self.Shooting` bShooting))

(fn `Shoot`
  (bind (_returnvalue_location _returnvalue_rotation) (`KismetMathLibrary.BreakTransform` (`SceneComponent.K2_GetComponentToWorld` (`self.Scene`))))
  (bind _returnvalue (`|SpawnActorFromClass` "/Game/Blueprints/Weapons/Bullets/BP_Bullet.BP_Bullet_C" (`KismetMathLibrary.MakeTransform` _returnvalue_location _returnvalue_rotation (2.0 2.0 2.0)) "Undefined" "OverrideRootScale" null null))
  (set `/Game/Blueprints/Weapons/Bullets/BP_Bullet.Speed` (`self.BulletSpeed`) _returnvalue)
  (set `/Game/Blueprints/Weapons/Bullets/BP_Bullet.Damage` (`self.Damage`) _returnvalue)
  (`GameplayStatics.PlaySoundAtLocation` "/Game/Assets/Audio/Audio/SoundEffects/Weapons/SMGShoot.SMGShoot" (`self.K2_GetActorLocation`) (struct) 1.0 1.0 0.0 null null null))

(fn `UserConstructionScript`)