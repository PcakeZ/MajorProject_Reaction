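; VR player clone that replays recorded headset, controller and input samples from LoadData, stepped by VRGameMode's play and read-sample events.
; Tick blends the hands and head hitbox with the current sample's transforms.
; Each sample edge-detects triggers, joysticks and grips to fire weapons, swap hand-attached weapon actors via radial menus, and run navmesh-projected teleport targeting.
; It also takes damage, with a brief invulnerability window after each hit.
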(event `self.ReceiveBeginPlay`
  ;[1 1 1] Begin Play
  ;;[1 1 1] Set Varibles
  (bind _asvrgame_mode (cast `/Game/Blueprints/Player/VRGamemode` (`GameplayStatics.GetGameMode`)))
  (set `self.VRGameMode` _asvrgame_mode)
  (bind _asw_hand_menu (cast `/Game/Widgets/W_HandMenu` (`WidgetComponent.GetUserWidgetObject` (`self.HandMenu_R`))))
  (set `self.HandMenuWidget_R` _asw_hand_menu)
  (bind _asw_hand_menu_2 (cast `/Game/Widgets/W_HandMenu` (`WidgetComponent.GetUserWidgetObject` (`self.HandMenu_L`))))
  (set `self.HandMenuWidget_L` _asw_hand_menu_2)
  (set `self.StartLocation` (`self.GetTransform`))
  (add `/Game/Blueprints/Player/VRGamemode.ReadSample` (`self.VRGameMode`) (delegate `ReadSample`))
  (add `/Game/Blueprints/Player/VRGamemode.PlaySample` (`self.VRGameMode`) (delegate `PlayerSamples`))
  (`KismetSystemLibrary.Delay` 0.05)
  (`self.Change Weapons` true (`self.CurrentWeaponRight`))
  (`self.Change Weapons` false (`self.CurrentWeaponLeft`)))

(event `self.ReceiveTick`
  (params (DeltaSeconds :type "Float (single-precision)"))
  (bind (_controlerr _controlerl _headset _weapontyper _weapontypel _rtrigger _ltrigger _rjoystickpressed _ljoystickpressed _rgrip _lgrip _rselectedarea _lselectedarea) (break `/Game/Blueprints/Player/PlayerSavedData` (`|GetArrayItem` (`self.LoadData`) (`self.LoadDataInt`))))
  ;[1 1 1] Tick
  ;;[1 1 0] Lerp Hand Positions
  (`SceneComponent.K2_SetWorldTransform` (`self.LerpedHand_R`) (`KismetMathLibrary.TLerp` _controlerr (`SceneComponent.K2_GetComponentToWorld` (`self.LerpedHand_R`)) (* (`GameplayStatics.GetWorldDeltaSeconds`) 20.0)) false false)
  (`SceneComponent.K2_SetWorldTransform` (`self.LerpedHand_L`) (`KismetMathLibrary.TLerp` _controlerl (`SceneComponent.K2_GetComponentToWorld` (`self.LerpedHand_L`)) (* (`GameplayStatics.GetWorldDeltaSeconds`) 20.0)) false false)
  (`SceneComponent.K2_SetWorldTransform` (`self.HeadHitbox`) (`KismetMathLibrary.TLerp` _headset (`SceneComponent.K2_GetComponentToWorld` (`self.HeadHitbox`)) (* (`GameplayStatics.GetWorldDeltaSeconds`) 20.0)) false false))

(event `PlayerSamples`
  (bind _handleft (`self.HandLeft`))
  (bind _handmenuwidget_l (`self.HandMenuWidget_L`))
  (bind _handmenuwidget_r (`self.HandMenuWidget_R`))
  (bind _handleft_2 (`self.HandLeft`))
  (bind _currentweaponleft (`self.CurrentWeaponLeft`))
  (bind _handright (`self.HandRight`))
  (bind _currentweaponright (`self.CurrentWeaponRight`))
  (bind _handright_2 (`self.HandRight`))
  (bind _selectedarea (`/Game/Widgets/W_HandMenu.SelectedArea` _handmenuwidget_l))
  (bind _selectedarea_2 (`/Game/Widgets/W_HandMenu.SelectedArea` _handmenuwidget_r))
  (bind (_controlerr _controlerl _headset _weapontyper _weapontypel _rtrigger _ltrigger _rjoystickpressed _ljoystickpressed _rgrip _lgrip _rselectedarea _lselectedarea) (break `/Game/Blueprints/Player/PlayerSavedData` (`|GetArrayItem` (`self.LoadData`) (`self.LoadDataInt`))))
  (bind _output (`|GetArrayItem` (`self.HandMenuLocked`) (`KismetMathLibrary.Conv_ByteToInt` _selectedarea_2)))
  (bind _output_2 (`|GetArrayItem` (`self.HandMenuLocked`) (`KismetMathLibrary.Conv_ByteToInt` _selectedarea)))
  ;[1 1 1] Tick
  (set `self.PlayingSample` true)
  (`|ExecutionSequence` :!label _label
    (:`then_0`
      (set `/Game/Widgets/W_HandMenu.SelectedArea` _lselectedarea (`self.HandMenuWidget_L`))
      (set `/Game/Widgets/W_HandMenu.SelectedArea` _rselectedarea (`self.HandMenuWidget_R`))
      (set `self.CurrentWeaponRight` _weapontyper)
      (set `self.CurrentWeaponLeft` _weapontypel))
    (:`then_1`
      (if (!= (`self.TriggerDown_R`) _rtrigger)
        ;;[1 0 0] Shooting
        (if _rtrigger
          (set `self.TriggerDown_R` true)
          (switch `/Game/Blueprints/Enums/WeaponTypes` _currentweaponright
            (:`NewEnumerator0`
              (bind _asbp_pistol (cast `/Game/Blueprints/Weapons/BP_Pistol` _handright))
              (`/Game/Blueprints/Weapons/BP_Pistol.Shoot` _asbp_pistol)
              (set `self.Shot_R` true))
            (:`NewEnumerator2`
              (bind _asbp_smg (cast `/Game/Blueprints/Weapons/BP_SMG` _handright))
              (`/Game/Blueprints/Weapons/BP_SMG.IsShooting` _asbp_smg true)
              (set `self.Shot_R` true))
            (:`NewEnumerator3`
              (bind _asbp_shotgun (cast `/Game/Blueprints/Weapons/BP_Shotgun` _handright))
              (`/Game/Blueprints/Weapons/BP_Shotgun.Shoot` _asbp_shotgun)
              (set `self.Shot_R` true))
            (:`NewEnumerator4`
              (bind _asbp_laser_gun (cast `/Game/Blueprints/Weapons/BP_LaserGun` _handright))
              (`/Game/Blueprints/Weapons/BP_LaserGun.StartFire` _asbp_laser_gun true)
              (set `self.Shot_R` true))
            (:`NewEnumerator5`
              (bind _asbp_grenade_launcher (cast `/Game/Blueprints/Weapons/BP_GrenadeLauncher` _handright))
              (`/Game/Blueprints/Weapons/BP_GrenadeLauncher.Shoot` _asbp_grenade_launcher)
              (set `self.Shot_R` true))
            (:`NewEnumerator6`
              (bind _asbp_pulse_gun (cast `/Game/Blueprints/Weapons/BP_PulseGun` _handright))
              (`/Game/Blueprints/Weapons/BP_PulseGun.IsShooting` _asbp_pulse_gun true)
              (set `self.Shot_R` true)))
          (else
            (set `self.TriggerDown_R` false)
            (switch `/Game/Blueprints/Enums/WeaponTypes` _currentweaponright
              (:`NewEnumerator2`
                (bind _asbp_smg_2 (cast `/Game/Blueprints/Weapons/BP_SMG` _handright_2))
                (`/Game/Blueprints/Weapons/BP_SMG.IsShooting` _asbp_smg_2 false)
                (set `self.Shot_R` false))
              (:`NewEnumerator4`
                (bind _asbp_laser_gun_2 (cast `/Game/Blueprints/Weapons/BP_LaserGun` _handright_2))
                (`/Game/Blueprints/Weapons/BP_LaserGun.StartFire` _asbp_laser_gun_2 false)
                (set `self.Shot_R` false))
              (:`NewEnumerator6`
                (bind _asbp_pulse_gun_2 (cast `/Game/Blueprints/Weapons/BP_PulseGun` _handright_2))
                (`/Game/Blueprints/Weapons/BP_PulseGun.IsShooting` _asbp_pulse_gun_2 false)
                (set `self.Shot_R` false)))))))
    (:`then_2`
      (if (!= (`self.TriggerDown_L`) _ltrigger)
        ;;[1 0 0] Shooting
        (if _ltrigger
          (set `self.TriggerDown_L` true)
          (switch `/Game/Blueprints/Enums/WeaponTypes` _currentweaponleft
            (:`NewEnumerator0`
              (bind _asbp_pistol_2 (cast `/Game/Blueprints/Weapons/BP_Pistol` _handleft))
              (`/Game/Blueprints/Weapons/BP_Pistol.Shoot` _asbp_pistol_2)
              (set `self.Shot_L` true))
            (:`NewEnumerator2`
              (bind _asbp_smg_3 (cast `/Game/Blueprints/Weapons/BP_SMG` _handleft))
              (`/Game/Blueprints/Weapons/BP_SMG.IsShooting` _asbp_smg_3 true)
              (set `self.Shot_L` true))
            (:`NewEnumerator3`
              (bind _asbp_shotgun_2 (cast `/Game/Blueprints/Weapons/BP_Shotgun` _handleft))
              (`/Game/Blueprints/Weapons/BP_Shotgun.Shoot` _asbp_shotgun_2)
              (set `self.Shot_L` true))
            (:`NewEnumerator4`
              (bind _asbp_laser_gun_3 (cast `/Game/Blueprints/Weapons/BP_LaserGun` _handleft))
              (`/Game/Blueprints/Weapons/BP_LaserGun.StartFire` _asbp_laser_gun_3 true)
              (set `self.Shot_L` true))
            (:`NewEnumerator5`
              (bind _asbp_grenade_launcher_2 (cast `/Game/Blueprints/Weapons/BP_GrenadeLauncher` _handleft))
              (`/Game/Blueprints/Weapons/BP_GrenadeLauncher.Shoot` _asbp_grenade_launcher_2)
              (set `self.Shot_L` true))
            (:`NewEnumerator6`
              (bind _asbp_pulse_gun_3 (cast `/Game/Blueprints/Weapons/BP_PulseGun` _handleft))
              (`/Game/Blueprints/Weapons/BP_PulseGun.IsShooting` _asbp_pulse_gun_3 true)
              (set `self.Shot_L` true)))
          (else
            (set `self.TriggerDown_L` false)
            (switch `/Game/Blueprints/Enums/WeaponTypes` _currentweaponleft
              (:`NewEnumerator2`
                (bind _asbp_smg_4 (cast `/Game/Blueprints/Weapons/BP_SMG` _handleft_2))
                (`/Game/Blueprints/Weapons/BP_SMG.IsShooting` _asbp_smg_4 false)
                (set `self.Shot_L` false))
              (:`NewEnumerator4`
                (bind _asbp_laser_gun_4 (cast `/Game/Blueprints/Weapons/BP_LaserGun` _handleft_2))
                (`/Game/Blueprints/Weapons/BP_LaserGun.StartFire` _asbp_laser_gun_4 false)
                (set `self.Shot_L` false))
              (:`NewEnumerator6`
                (bind _asbp_pulse_gun_4 (cast `/Game/Blueprints/Weapons/BP_PulseGun` _handleft_2))
                (`/Game/Blueprints/Weapons/BP_PulseGun.IsShooting` _asbp_pulse_gun_4 false)
                (set `self.Shot_L` false)))))))
    (:`then_3`
      ;;[1 0.9615 0] Weapon Select Right
      (if (!= (`self.JoystickDown_R`) _rjoystickpressed)
        (if _rjoystickpressed
          (bind _output_get (set `self.JoystickDown_R` true))
          (set `/Game/Widgets/W_HandMenu.Visible` _output_get _handmenuwidget_r)
          (else
            (bind _output_get_2 (set `self.JoystickDown_R` false))
            (set `/Game/Widgets/W_HandMenu.Visible` _output_get_2 _handmenuwidget_r)
            (switch `/Game/Blueprints/Enums/Enum_HandMenuSelected` _selectedarea_2
              (:`NewEnumerator0`
                (if _output
                  (`self.Change Weapons` true)))
              (:`NewEnumerator1`
                (if _output
                  (`self.Change Weapons` true "NewEnumerator0")))
              (:`NewEnumerator2`
                (if _output
                  (`self.Change Weapons` true "NewEnumerator2")))
              (:`NewEnumerator3`
                (if _output
                  (`self.Change Weapons` true "NewEnumerator3")))
              (:`NewEnumerator4`
                (if _output
                  (`self.Change Weapons` true "NewEnumerator4")))
              (:`NewEnumerator5`
                (if _output
                  (`self.Change Weapons` true "NewEnumerator5")))
              (:`NewEnumerator6`
                (if _output
                  (`self.Change Weapons` true "NewEnumerator6"))))))))
    (:`then_4`
      (if (!= (`self.JoystickDown_L`) _ljoystickpressed)
        ;;[1 0.9744 0] Weapon Select Left
        (if _ljoystickpressed
          (bind _output_get_3 (set `self.JoystickDown_L` true))
          (set `/Game/Widgets/W_HandMenu.Visible` _output_get_3 _handmenuwidget_l)
          (else
            (bind _output_get_4 (set `self.JoystickDown_L` false))
            (set `/Game/Widgets/W_HandMenu.Visible` _output_get_4 _handmenuwidget_l)
            (switch `/Game/Blueprints/Enums/Enum_HandMenuSelected` _selectedarea
              (:`NewEnumerator0`
                (if _output_2
                  (`self.Change Weapons` false)))
              (:`NewEnumerator1`
                (if _output_2
                  (`self.Change Weapons` false "NewEnumerator0")))
              (:`NewEnumerator2`
                (if _output_2
                  (`self.Change Weapons` false "NewEnumerator2")))
              (:`NewEnumerator3`
                (if _output_2
                  (`self.Change Weapons` false "NewEnumerator3")))
              (:`NewEnumerator4`
                (if _output_2
                  (`self.Change Weapons` false "NewEnumerator4")))
              (:`NewEnumerator5`
                (if _output_2
                  (`self.Change Weapons` false "NewEnumerator5")))
              (:`NewEnumerator6`
                (if _output_2
                  (`self.Change Weapons` false "NewEnumerator6"))))))))
    (:`then_5`
      (if (!= (`self.bTeleportHold_R`) _rgrip)
        (if _rgrip
          ;;[0 1 0.09904] Teleport
          (set `self.bTeleportHold_R` true)
          (else
            (set `self.bTeleportHold_R` false)
            (set `self.IsTeleporting` true)
            (set `self.TPLocation` (`self.TPLocation_R`))
            (`SceneComponent.SetVisibility` (`self.TeleportMarket_R`) false false)))))
    (:`then_6`
      (if (!= (`self.bTeleportHold_L`) _lgrip)
        (if _lgrip
          (set `self.bTeleportHold_L` true)
          (else
            (set `self.bTeleportHold_L` false)
            (set `self.IsTeleporting` true)
            (set `self.TPLocation` (`self.TPLocation_L`))
            (`SceneComponent.SetVisibility` (`self.TeleportMarket_L`) false false)))))
    (:`then_7`
      ;;[0 0.3314 1] GetTPLocation
      (if (`self.bTeleportHold_R`)
        (`self.GripTeleport` (`SceneComponent.K2_GetComponentLocation` (`self.RightTPPos1`)) 200.0 true))
      (if (`self.bTeleportHold_L`)
        (`self.GripTeleport` (`SceneComponent.K2_GetComponentLocation` (`self.LeftTPPos1`)) 200.0)))
    (:`then_8`
      (if (`self.PlayingSample`)
        (`/Engine/EditorBlueprintResources/StandardMacros.IncrementInt` (`self.LoadDataInt`)
          (:`  `
            (set `self.PlayingSample` false)))))))

(event `ReadSample`
  (params (Sample :type Integer))
  ;[1 1 1] Tick
  (set `self.LoadDataInt` Sample)
  (goto _label))

(event `self.ReceiveDestroyed`
  ;[1 1 1] Tick
  (`self.K2_DestroyActor` (`self.HandRight`))
  (`self.K2_DestroyActor` (`self.HandLeft`)))

(event `self.ReceiveAnyDamage`
  (params (Damage :type "Float (single-precision)") (DamageType :type "DamageType Object Reference") (InstigatedBy :type "Controller Object Reference") (DamageCauser :type "Actor Object Reference"))
  ;[1 1 1] Tick
  ;;[1 0.02604 0.02604] Take Damage
  (if (not (`self.IsInvulnerable`))
    (set `self.Health` (- (`self.Health`) Damage))
    (set `self.IsInvulnerable` true)
    (`GameplayStatics.PlaySound2D` "/Game/Assets/Audio/Audio/SoundEffects/PlayerHit.PlayerHit" 1.0 1.0 0.0 null null)
    (`KismetSystemLibrary.Delay` (`self.HitInvulnerability`))
    (set `self.IsInvulnerable` false)))

(fn `Change Weapons`
  (params (RHand :type Boolean) (WeaponType :type "/Game/Blueprints/Enums/WeaponTypes Enum" :default "NewEnumerator1"))
  (bind _handleft (`self.HandLeft`))
  (bind _handright (`self.HandRight`))
  (bind (_returnvalue_location _returnvalue_rotation) (`KismetMathLibrary.BreakTransform` (`SceneComponent.K2_GetComponentToWorld` (`self.LerpedHand_L`))))
  (bind (_returnvalue_location_2 _returnvalue_rotation_2) (`KismetMathLibrary.BreakTransform` (`SceneComponent.K2_GetComponentToWorld` (`self.LerpedHand_R`))))
  (bind (_controlerr _controlerl _headset _weapontyper _weapontypel) (break `/Game/Blueprints/Player/PlayerSavedData` (`|GetArrayItem` (`self.LoadData`) (`self.LoadDataInt`))))
  (if RHand
    (set `self.CurrentWeaponRight` _weapontyper)
    (`/Engine/EditorBlueprintResources/StandardMacros.IsValid` _handright
      (:`Is Valid`
        (`self.K2_DestroyActor` _handright))
      (:`Is Not Valid`
        _))
    ;[1 1 1] Create Weapon (Right Hand)
    (switch `/Game/Blueprints/Enums/WeaponTypes` (`self.CurrentWeaponRight`)
      (:`NewEnumerator1`
        (bind _returnvalue (`|SpawnActorFromClass` "/Game/Blueprints/Weapons/BP_Sheild.BP_Sheild_C" (`KismetMathLibrary.MakeTransform` _returnvalue_location_2 _returnvalue_rotation_2) "Undefined" "OverrideRootScale" null null))
        (set `self.HandRight` _returnvalue))
      (:`NewEnumerator0`
        (bind _returnvalue_2 (`|SpawnActorFromClass` "/Game/Blueprints/Weapons/BP_Pistol.BP_Pistol_C" (`KismetMathLibrary.MakeTransform` _returnvalue_location_2 _returnvalue_rotation_2) "Undefined" "OverrideRootScale" null null))
        (set `self.HandRight` _returnvalue_2))
      (:`NewEnumerator2`
        (bind _returnvalue_3 (`|SpawnActorFromClass` "/Game/Blueprints/Weapons/BP_SMG.BP_SMG_C" (`KismetMathLibrary.MakeTransform` _returnvalue_location_2 _returnvalue_rotation_2) "Undefined" "OverrideRootScale" null null))
        (set `self.HandRight` _returnvalue_3))
      (:`NewEnumerator3`
        (bind _returnvalue_4 (`|SpawnActorFromClass` "/Game/Blueprints/Weapons/BP_Shotgun.BP_Shotgun_C" (`KismetMathLibrary.MakeTransform` _returnvalue_location_2 _returnvalue_rotation_2) "Undefined" "OverrideRootScale" null null))
        (set `self.HandRight` _returnvalue_4))
      (:`NewEnumerator4`
        (bind _returnvalue_5 (`|SpawnActorFromClass` "/Game/Blueprints/Weapons/BP_LaserGun.BP_LaserGun_C" (`KismetMathLibrary.MakeTransform` _returnvalue_location_2 _returnvalue_rotation_2) "Undefined" "OverrideRootScale" null null))
        (set `self.HandRight` _returnvalue_5))
      (:`NewEnumerator5`
        (bind _returnvalue_6 (`|SpawnActorFromClass` "/Game/Blueprints/Weapons/BP_GrenadeLauncher.BP_GrenadeLauncher_C" (`KismetMathLibrary.MakeTransform` _returnvalue_location_2 _returnvalue_rotation_2) "Undefined" "OverrideRootScale" null null))
        (set `self.HandRight` _returnvalue_6))
      (:`NewEnumerator6`
        (bind _returnvalue_7 (`|SpawnActorFromClass` "/Game/Blueprints/Weapons/BP_PulseGun.BP_PulseGun_C" (`KismetMathLibrary.MakeTransform` _returnvalue_location_2 _returnvalue_rotation_2) "Undefined" "OverrideRootScale" null null))
        (set `self.HandRight` _returnvalue_7)))
    (`self.K2_AttachToComponent` (`self.HandRight`) (`self.LerpedHand_R`) "None" "KeepWorld" "KeepWorld" "KeepWorld" true)
    (else
      (set `self.CurrentWeaponLeft` _weapontypel)
      (`/Engine/EditorBlueprintResources/StandardMacros.IsValid` _handleft
        (:`Is Valid`
          (`self.K2_DestroyActor` _handleft))
        (:`Is Not Valid`
          _))
      ;[1 1 1] Create Weapon (Left Hand)
      (switch `/Game/Blueprints/Enums/WeaponTypes` (`self.CurrentWeaponLeft`)
        (:`NewEnumerator1`
          (bind _returnvalue_8 (`|SpawnActorFromClass` "/Game/Blueprints/Weapons/BP_Sheild.BP_Sheild_C" (`KismetMathLibrary.MakeTransform` _returnvalue_location _returnvalue_rotation) "Undefined" "OverrideRootScale" null null))
          (set `self.HandLeft` _returnvalue_8))
        (:`NewEnumerator0`
          (bind _returnvalue_9 (`|SpawnActorFromClass` "/Game/Blueprints/Weapons/BP_Pistol.BP_Pistol_C" (`KismetMathLibrary.MakeTransform` _returnvalue_location _returnvalue_rotation) "Undefined" "OverrideRootScale" null null))
          (set `self.HandLeft` _returnvalue_9))
        (:`NewEnumerator2`
          (bind _returnvalue_10 (`|SpawnActorFromClass` "/Game/Blueprints/Weapons/BP_SMG.BP_SMG_C" (`KismetMathLibrary.MakeTransform` _returnvalue_location _returnvalue_rotation) "Undefined" "OverrideRootScale" null null))
          (set `self.HandLeft` _returnvalue_10))
        (:`NewEnumerator3`
          (bind _returnvalue_11 (`|SpawnActorFromClass` "/Game/Blueprints/Weapons/BP_Shotgun.BP_Shotgun_C" (`KismetMathLibrary.MakeTransform` _returnvalue_location _returnvalue_rotation) "Undefined" "OverrideRootScale" null null))
          (set `self.HandLeft` _returnvalue_11))
        (:`NewEnumerator4`
          (bind _returnvalue_12 (`|SpawnActorFromClass` "/Game/Blueprints/Weapons/BP_LaserGun.BP_LaserGun_C" (`KismetMathLibrary.MakeTransform` _returnvalue_location _returnvalue_rotation) "Undefined" "OverrideRootScale" null null))
          (set `self.HandLeft` _returnvalue_12))
        (:`NewEnumerator5`
          (bind _returnvalue_13 (`|SpawnActorFromClass` "/Game/Blueprints/Weapons/BP_GrenadeLauncher.BP_GrenadeLauncher_C" (`KismetMathLibrary.MakeTransform` _returnvalue_location _returnvalue_rotation) "Undefined" "OverrideRootScale" null null))
          (set `self.HandLeft` _returnvalue_13))
        (:`NewEnumerator6`
          (bind _returnvalue_14 (`|SpawnActorFromClass` "/Game/Blueprints/Weapons/BP_PulseGun.BP_PulseGun_C" (`KismetMathLibrary.MakeTransform` _returnvalue_location _returnvalue_rotation) "Undefined" "OverrideRootScale" null null))
          (set `self.HandLeft` _returnvalue_14)))
      (`self.K2_AttachToComponent` (`self.HandLeft`) (`self.LerpedHand_L`) "None" "KeepWorld" "KeepWorld" "KeepWorld" true))))

(fn `ChangeEquipment`
  (params (RHand :type Boolean)))

(fn `FindTPLocation`
  (params (LaunchSpeed :type "Float (double-precision)"))
  (bind _motioncontroller_l (`self.MotionController_L`))
  (bind _outhit (`GameplayStatics.Blueprint_PredictProjectilePath_ByTraceChannel` (`SceneComponent.K2_GetComponentLocation` _motioncontroller_l) (* (`SceneComponent.GetForwardVector` _motioncontroller_l) LaunchSpeed) true 0.0 "ECC_Visibility" true))
  (bind (_projectedlocation _returnvalue) (`NavigationSystemV1.K2_ProjectPointToNavigation` (`.Location` (`GameplayStatics.BreakHitResult` _outhit))))
  (if _returnvalue
    (`KismetSystemLibrary.DrawDebugCylinder` _projectedlocation (`KismetMathLibrary.MakeVector` (.x _projectedlocation) (.y _projectedlocation) (+ (.z _projectedlocation) 30.0)) 30.0 12 (struct :`R` 1.0 :`A` 1.0))
    (set `self.TPLocation_R` _projectedlocation)))

(fn `GripTeleport`
  (params (TracePos :type "Vector Structure") (DownTraceDistance :type "Float (double-precision)") (RHand :type Boolean))
  (returns (TPPos :type "Vector Structure"))
  (locals (bRHand :type Boolean))
  (bind _brhand (`local.bRHand`))
  (bind _teleportmarket_r (`self.TeleportMarket_R`))
  (bind _teleportmarket_l (`self.TeleportMarket_L`))
  (set `local.bRHand` RHand)
  (bind (_outhit _returnvalue) (`KismetSystemLibrary.LineTraceSingle` TracePos (- TracePos (`KismetMathLibrary.MakeVector` 0.0 0.0 DownTraceDistance)) "TraceTypeQuery1"))
  (if _returnvalue
    (bind (_projectedlocation _returnvalue_2) (`NavigationSystemV1.K2_ProjectPointToNavigation` (`.Location` (`GameplayStatics.BreakHitResult` _outhit))))
    (if _returnvalue_2
      (if _brhand
        (`SceneComponent.SetVisibility` _teleportmarket_r true false)
        (`SceneComponent.K2_SetWorldLocation` _teleportmarket_r _projectedlocation false false)
        (else
          (`SceneComponent.SetVisibility` _teleportmarket_l true false)
          (`SceneComponent.K2_SetWorldLocation` _teleportmarket_l _projectedlocation false false)))
      (return _projectedlocation)
      (else
        (if _brhand
          (`SceneComponent.SetVisibility` (`self.TeleportMarket_R`) false false)
          (else
            (`SceneComponent.SetVisibility` (`self.TeleportMarket_L`) false false)))
        (return (`NavigationSystemV1.K2_ProjectPointToNavigation` (`SceneComponent.K2_GetComponentLocation` (`self.HeadHitbox`))))))))

(fn `SetHandMenu`
  (params (X :type "Float (double-precision)") (Y :type "Float (double-precision)"))
  (returns (FingerPosition1 :type "/Game/Blueprints/Enums/Enum_HandMenuSelected Enum"))
  (locals (XCoord :type "Float (double-precision)") (YCoord :type "Float (double-precision)") (Angle :type "Float (double-precision)") (FingerPosition :type "/Game/Blueprints/Enums/Enum_HandMenuSelected Enum"))
  (bind _xcoord (`local.XCoord`))
  (bind _ycoord (`local.YCoord`))
  (bind _angle (`local.Angle`))
  ;[1 1 1] Get touchpad Angle
  (set `local.XCoord` X)
  (set `local.YCoord` Y)
  (if (or (!= 0.0 _ycoord) (!= 0.0 _xcoord))
    (bind _output_get (set `local.Angle` (- 360.0 (+ (`KismetMathLibrary.DegAtan2` _ycoord _xcoord) 270.0))))
    (if (< _output_get 0.0)
      (set `local.Angle` (+ (- 90.0 (* (`local.Angle`) -1.0)) 270.0)))
    ;[1 1 1] Set Selected Position
    (if (and (< (`KismetMathLibrary.Abs` (`local.YCoord`)) 0.3) (< (`KismetMathLibrary.Abs` (`local.XCoord`)) 0.3))
      (bind _output_get_2 (set `local.FingerPosition` "NewEnumerator0"))
      (return _output_get_2)
      (elif (or (>= _angle 331.0) (<= _angle 30.0))
        (bind _output_get_3 (set `local.FingerPosition` "NewEnumerator1"))
        (return _output_get_3)
        (else
          (switch `int` (`KismetMathLibrary.Round` (- (/ (+ _angle -30.0) 60.0) 0.5))
            (:`0`
              (set `local.FingerPosition` "NewEnumerator2"))
            (:`1`
              (set `local.FingerPosition` "NewEnumerator3"))
            (:`2`
              (set `local.FingerPosition` "NewEnumerator4"))
            (:`3`
              (set `local.FingerPosition` "NewEnumerator5"))
            (:`4`
              (set `local.FingerPosition` "NewEnumerator6")))
          (return (`local.FingerPosition`)))))))

(fn `UserConstructionScript`)