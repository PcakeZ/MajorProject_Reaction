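; VR game mode Blueprint that starts and resets a loop in which clones of the player are spawned.
; It caches the VRPawn on BeginPlay and tracks the loop state through GameOn, set by StartGame and cleared by LoopReset.
; StartGame spawns up to three VRClone actors at the player's start location, handing each a saved data array.
; The checks are nested, so each clone requires the previous slot to hold data.
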(event `self.ReceiveBeginPlay`
  (bind _asvrpawn (cast `/Game/Blueprints/Player/VRPawn` (`GameplayStatics.GetPlayerPawn` 0)))
  (set `self.Player` _asvrpawn))

(event `self.ReceiveTick`
  (params (DeltaSeconds :type "Float (single-precision)")))

(event `/Game/Blueprints/Interface/I_GameFlow.StartGame`
  (bind _clone3 (`self.Clone3`))
  (bind _clone2 (`self.Clone2`))
  (bind _clone1 (`self.Clone1`))
  (set `self.GameOn` true)
  (if (> (`KismetArrayLibrary.Array_Length` _clone1) 1)
    (`KismetSystemLibrary.PrintString` (`KismetStringLibrary.Concat_StrStr` "CLONE MADE: ") true true (struct :`G` 0.66 :`B` 1.0 :`A` 1.0) 10.0)
    (bind _returnvalue (`|SpawnActorFromClass` "/Game/Blueprints/Player/VRClone.VRClone_C" (`/Game/Blueprints/Player/VRPawn.StartLocation` (`self.Player`)) "AlwaysSpawn" "OverrideRootScale" null null))
    (set `/Game/Blueprints/Player/VRClone.SavedData` _clone1 _returnvalue)
    (if (> (`KismetArrayLibrary.Array_Length` _clone2) 1)
      (`KismetSystemLibrary.PrintString` (`KismetStringLibrary.Concat_StrStr` "CLONE MADE: ") true true (struct :`G` 0.66 :`B` 1.0 :`A` 1.0) 10.0)
      (bind _returnvalue_2 (`|SpawnActorFromClass` "/Game/Blueprints/Player/VRClone.VRClone_C" (`/Game/Blueprints/Player/VRPawn.StartLocation` (`self.Player`)) "AlwaysSpawn" "OverrideRootScale" null null))
      (set `/Game/Blueprints/Player/VRClone.SavedData` _clone2 _returnvalue_2)
      (if (> (`KismetArrayLibrary.Array_Length` _clone3) 1)
        (`KismetSystemLibrary.PrintString` (`KismetStringLibrary.Concat_StrStr` "CLONE MADE: ") true true (struct :`G` 0.66 :`B` 1.0 :`A` 1.0) 10.0)
        (bind _returnvalue_3 (`|SpawnActorFromClass` "/Game/Blueprints/Player/VRClone.VRClone_C" (`/Game/Blueprints/Player/VRPawn.StartLocation` (`self.Player`)) "AlwaysSpawn" "OverrideRootScale" null null))
        (set `/Game/Blueprints/Player/VRClone.SavedData` _clone3 _returnvalue_3)))))

(event `/Game/Blueprints/Interface/I_GameFlow.LoopReset`
  (set `self.GameOn` false))

(fn `UserConstructionScript`)