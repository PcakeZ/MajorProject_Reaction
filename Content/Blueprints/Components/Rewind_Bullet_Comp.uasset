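; Bullet component for a rewind system that records, plays back and scrubs its BP_Bullet owner through sample events bound on VRGameMode.
; Recording keeps a rolling array of mesh transform, destroyed flag and trail distance, capped by RecordTime.
; Playback and scrubbing reapply those samples, hiding the bullet for times before its recording starts.
; Destroy only hides and flags the bullet; Recording destroys the actor later, based on the recorded flag.
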(event `self.ReceiveBeginPlay`
  (bind _returnvalue (`self.GetOwner`))
  (bind _vrgamemode (`self.VRGameMode`))
  ;[1 1 1] Begin Play
  (bind _asvrgame_mode (cast `/Game/Blueprints/Player/VRGamemode` (`GameplayStatics.GetGameMode`)))
  (set `self.VRGameMode` _asvrgame_mode)
  (set `self.SamplesPerSec` (`/Game/Blueprints/Player/VRGamemode.SamplesPerSecond` _asvrgame_mode))
  (set `self.RecordTime` (`/Game/Blueprints/Player/VRGamemode.RecordTime` _asvrgame_mode))
  (add `/Game/Blueprints/Player/VRGamemode.ReadSample` _vrgamemode (delegate `ReadSample`))
  (add `/Game/Blueprints/Player/VRGamemode.PlaySample` _vrgamemode (delegate `PlaySample`))
  (add `/Game/Blueprints/Player/VRGamemode.RecordSample` (`self.VRGameMode`) (delegate `Recording`))
  (bind _asbp_bullet (cast `/Game/Blueprints/Weapons/Bullets/BP_Bullet` _returnvalue)
    (:`then`
      (set `self.BulletActor` _asbp_bullet)
      (set `self.Bullet` (`/Game/Blueprints/Weapons/Bullets/BP_Bullet.StaticMesh` _asbp_bullet)))
    (:`CastFailed`
      (`Actor.K2_DestroyActor` _returnvalue))))

(event `Recording`
  (bind _array (`self.Array`))
  (bind (_output_trans _output_destoryed) (break `/Game/DataAndStructs/Struct_Rewind_Bullet` (`|GetArrayItem` (`self.Array`) (`KismetMathLibrary.FTrunc` (- (`self.RecordTime`) 1.0)))))
  ;[1 1 1] Recording
  (if _output_destoryed
    (`Actor.K2_DestroyActor` (`self.GetOwner`))
    (else
      (if (> (- (`KismetArrayLibrary.Array_Length` (`self.Array`)) 1) (`KismetMathLibrary.FTrunc` (`self.RecordTime`)))
        (`KismetArrayLibrary.Array_Remove` _array))
      (`KismetArrayLibrary.Array_Add` _array (make `/Game/DataAndStructs/Struct_Rewind_Bullet` (`SceneComponent.K2_GetComponentToWorld` (`self.Bullet`)) (`self.Destoryed`) (`/Game/Blueprints/Weapons/Bullets/BP_Bullet.distanceTravel` (`self.BulletActor`)))))))

(event `PlaySample`
  (bind (_output_trans _output_destoryed _output_traillength) (break `/Game/DataAndStructs/Struct_Rewind_Bullet` (`|GetArrayItem` (`self.Array`) (`self.int`))))
  ;[1 1 1] Play & Scrub Recording
  (`/Engine/EditorBlueprintResources/StandardMacros.IncrementInt` (`self.int`)
    (:`  `
      (`SceneComponent.K2_SetWorldTransform` (`self.Bullet`) _output_trans false false :!label _label)
      (`Actor.SetActorHiddenInGame` (`self.GetOwner`) _output_destoryed)
      (set `/Game/Blueprints/Weapons/Bullets/BP_Bullet.distanceTravel` _output_traillength (`self.BulletActor`)))))

(event `ReadSample`
  (params (Sample :type Integer))
  (bind _returnvalue (- Sample (`KismetMathLibrary.FTrunc` (- (`self.RecordTime`) (`KismetMathLibrary.Conv_IntToDouble` (- (`KismetArrayLibrary.Array_Length` (`self.Array`)) 1))))))
  ;[1 1 1] Play & Scrub Recording
  (if (< _returnvalue 0)
    (`Actor.SetActorHiddenInGame` (`self.GetOwner`) true)
    (else
      (set `self.int` _returnvalue)
      (if (< (`self.int`) (`KismetArrayLibrary.Array_Length` (`self.Array`)))
        (goto _label)))))

(event `Destroy`
  ;[1 1 1] Set Object Destroy
  (`Actor.SetActorHiddenInGame` (`self.GetOwner`) true)
  (set `self.Destoryed` true))