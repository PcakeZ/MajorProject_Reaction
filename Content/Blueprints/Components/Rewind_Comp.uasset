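; Actor component that records its owner's transform history for a rewind mechanic driven by the VR pawn.
; It binds to the pawn's record, play and read events, storing delayed transform and physics samples capped by RecordTime by replacing the last entry.
; Playback teleports the owner to the indexed sample's transform, with read events setting the index; stored physics is unused.
; The periodic reset is empty and the replay-array setup is unconnected.
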(event `self.ReceiveBeginPlay`
  (bind _vrgamemode (`self.VRGameMode`))
  (bind _asvrpawn (cast `/Game/Blueprints/Player/VRPawn` (`GameplayStatics.GetPlayerPawn` 0)))
  (set `self.VRGameMode` _asvrpawn)
  (set `self.SamplesPerSec` (`/Game/Blueprints/Player/VRPawn.SamplesPerSecond` _asvrpawn))
  (set `self.RecordTime` (`/Game/Blueprints/Player/VRPawn.RecordTime` _asvrpawn))
  (add `/Game/Blueprints/Player/VRGamemode.ReadSample` _vrgamemode (delegate `ReadSample`))
  (add `/Game/Blueprints/Player/VRGamemode.PlaySample` _vrgamemode (delegate `PlaySample`))
  (add `/Game/Blueprints/Player/VRGamemode.RecordSample` _vrgamemode (delegate `Recording`)))

(event `Recording`
  (bind _array (`self.Array`))
  (bind _returnvalue (`KismetArrayLibrary.Array_Length` (`self.Array`)))
  (`KismetSystemLibrary.Delay` (`self.SamplesPerSec`))
  (if (> _returnvalue (`KismetMathLibrary.FTrunc` (`self.RecordTime`)))
    (`KismetArrayLibrary.Array_Remove` _array (- _returnvalue 1)))
  (`KismetArrayLibrary.Array_Add` _array (make `/Game/DataAndStructs/PhysicsStruct` (`Actor.GetTransform` (`self.GetOwner`)) (`self.Physics`))))

(event `self.ReceiveTick`
  (params (DeltaSeconds :type "Float (single-precision)"))
  (`|ExecutionSequence`
    (:`then_1`
      (`KismetSystemLibrary.Delay` 1.0)
      (`self.ResetObject`))))

(event `PlaySample`
  (bind _output_trans (break `/Game/DataAndStructs/PhysicsStruct` (`|GetArrayItem` (`self.Array`) (`self.int`))))
  (`KismetSystemLibrary.Delay` (`self.SamplesPerSec`))
  (`Actor.K2_SetActorTransform` (`self.GetOwner`) _output_trans false true :!label _label))

(event `ReadSample`
  (params (Sample :type Integer))
  (set `self.int` Sample)
  (goto _label))

(event `ResetObject`)