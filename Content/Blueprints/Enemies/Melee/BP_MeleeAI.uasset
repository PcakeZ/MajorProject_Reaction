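; BP_MeleeAI is a melee enemy that runs after the VR player.
; On BeginPlay it starts a looping running animation and caches the player's VRPawn.
; Each Tick it scales the animation play rate by its speed and reissues AIMoveTo toward the player's camera location.
; Any damage destroys it immediately, and the file contains no attack logic.
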(event `self.ReceiveBeginPlay`
  (`SkeletalMeshComponent.PlayAnimation` (`self.Mesh`) "/Game/Assets/OtherAssets/Mixamo/Running/Running_Anim_mixamo_com.Running_Anim_mixamo_com" true)
  (bind _asvrpawn (cast `/Game/Blueprints/Player/VRPawn` (`GameplayStatics.GetPlayerPawn` 0)))
  (set `self.Player` _asvrpawn))

(event `self.ReceiveTick`
  (params (DeltaSeconds :type "Float (single-precision)"))
  (`SkeletalMeshComponent.SetPlayRate` (`self.Mesh`) (/ (`KismetMathLibrary.VSize` (`self.GetVelocity`)) 250.0))
  (`|AIMoveTo` self (`SceneComponent.K2_GetComponentLocation` (`/Game/Blueprints/Player/VRPawn.Camera` (`self.Player`))) null))

(event `self.ReceiveAnyDamage`
  (params (Damage :type "Float (single-precision)") (DamageType :type "DamageType Object Reference") (InstigatedBy :type "Controller Object Reference") (DamageCauser :type "Actor Object Reference"))
  (`self.K2_DestroyActor`))

(fn `UserConstructionScript`)