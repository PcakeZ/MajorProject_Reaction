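; BP_CrawlAI is a crawling enemy that moves toward the VR player's start location.
; On BeginPlay it loops a crawl animation on its mesh and caches player pawn 0 as a VRPawn.
; Each Tick it scales the animation play rate to its velocity and reissues an AI MoveTo toward that pawn's StartLocation.
; It contains no attack or overlap logic.
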(event `self.ReceiveBeginPlay`
  (`SkeletalMeshComponent.PlayAnimation` (`self.Mesh`) "/Game/Assets/OtherAssets/Mixamo/Crawling/Running_Crawl__1__Anim_mixamo_com.Running_Crawl__1__Anim_mixamo_com" true)
  (bind _asvrpawn (cast `/Game/Blueprints/Player/VRPawn` (`GameplayStatics.GetPlayerPawn` 0)))
  (set `self.Player` _asvrpawn))

(event `self.ReceiveTick`
  (params (DeltaSeconds :type "Float (single-precision)"))
  (bind _startlocation_location (`KismetMathLibrary.BreakTransform` (`/Game/Blueprints/Player/VRPawn.StartLocation` (`self.Player`))))
  (`SkeletalMeshComponent.SetPlayRate` (`self.Mesh`) (/ (`KismetMathLibrary.VSize` (`self.GetVelocity`)) 250.0))
  (`|AIMoveTo` self _startlocation_location null))

(fn `UserConstructionScript`)