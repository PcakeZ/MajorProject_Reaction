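; BP_SimpleSpawner is an enemy spawner actor that repeatedly spawns AI at its own transform on a timer.
; Tick counts CurrentTimer down, spawns BP_CrawlAI or BP_MeleeAI depending on the Crawling flag, then resets to SpawnTime.
; StartGame and LoopReset toggle GameStarted, but its check is disconnected, so spawning runs from BeginPlay regardless of that flag.
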(event `self.ReceiveBeginPlay`
  (set `self.CurrentTimer` (`self.SpawnTime`)))

(event `self.ReceiveTick`
  (params (DeltaSeconds :type "Float (single-precision)"))
  (bind _output_get (set `self.CurrentTimer` (- (`self.CurrentTimer`) DeltaSeconds)))
  (if (< _output_get 0.0)
    (if (`self.Crawling`)
      (`|SpawnActorFromClass` "/Game/Blueprints/Enemies/Melee/BP_CrawlAI.BP_CrawlAI_C" (`self.GetTransform`) "Undefined" "OverrideRootScale" null null)
      (else
        (`|SpawnActorFromClass` "/Game/Blueprints/Enemies/Melee/BP_MeleeAI.BP_MeleeAI_C" (`self.GetTransform`) "Undefined" "OverrideRootScale" null null)))
    (set `self.CurrentTimer` (`self.SpawnTime`))))

(event `/Game/Blueprints/Interface/I_GameFlow.StartGame`
  (set `self.GameStarted` true)
  (set `self.CurrentTimer` (`self.SpawnTime`)))

(event `/Game/Blueprints/Interface/I_GameFlow.LoopReset`
  (set `self.GameStarted` false))

(fn `UserConstructionScript`)